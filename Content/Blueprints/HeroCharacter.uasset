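; Twin-stick shooter hero Character that moves on world axes and fires an attached weapon.
; Fire axis input past a deadzone sets control rotation and pulls the weapon trigger, otherwise releasing it.
; BeginPlay spawns the weapon onto the mesh's GunSocket and records the spawn transform in TwinStickGameMode.
; AffectHealth updates and prints health, and on death asks the game mode to respawn the player, then destroys weapon and hero.
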(event EventBeginPlay
  (bind _mesh (Variables|Character|GetMesh))
  (Utilities|FlowControl|Sequence
    (:then_0
      ;[1 1 1] Weapon Setup
      (bind _returnvalue (Game|SpawnActorfromClass "/Game/Actors/Blueprints/Weapon.Weapon_C" (Transformation|GetWorldTransform _mesh) "Undefined" 0 0))
      (bind _output_get (Variables|Default|SetWeapon _returnvalue))
      (Transformation|AttachComponentToComponent _output_get _mesh "GunSocket" "SnapToTarget" "SnapToTarget" "KeepWorld" true))
    (:then_1
      ;[1 1 1] SendSpawnToGameMode
      (bind _astwin_stick_game_mode (Utilities|Casting|CastToTwinStickGameMode (Game|GetGameMode)))
      (bind _output_get_2 (Variables|Default|SetGameMode _astwin_stick_game_mode))
      (Variables|/Game/TwinStickBP/Blueprints/Blueprints/TwinStickGameMode.TwinStickGameMode_C|SetPlayerSpawnTransform _output_get_2 (Transformation|GetActorTransform)))))

(event Collision|EventActorBeginOverlap
  (params (OtherActor :type Actor%20Object%20Reference)))

(event EventTick
  (params (DeltaSeconds :type Float%20%28single-precision%29)))

(event EventAffectHealth
  (params (Delta :type Float%20%28single-precision%29))
  ;[1 1 1] Health
  (Class|BaseCharacter|CalculateHealth Delta)
  (Development|PrintString (Utilities|String|ToString(Float) (Variables|Default|GetHealth)))
  (if (Variables|Default|GetisDead)
    (Default|RespawnPlayer (Variables|Default|GetGameMode))
    (Actor|DestroyActor (Variables|Default|GetWeapon))))

(event Input|AxisEvents|InputAxisMoveUp
  (params (AxisValue :type Float%20%28single-precision%29))
  ;[1 1 1] Movement
  (Pawn|Input|AddMovementInput "0.000000,1.000000, 0" AxisValue false))

(event Input|AxisEvents|InputAxisMoveRight
  (params (AxisValue :type Float%20%28single-precision%29))
  ;[1 1 1] Movement
  (Pawn|Input|AddMovementInput "1.000000,0.000000, 0" AxisValue false))

(event Input|AxisEvents|InputAxisFireUp
  (params (AxisValue :type Float%20%28single-precision%29))
  (bind _weapon (Variables|Default|GetWeapon))
  ;[1 1 1] Rotation
  (if (> (Math|Vector|VectorLength (Math|Vector|MakeVector (stale Input|AxisEvents|InputAxisFireRight AxisValue) AxisValue 0.0)) 0.25)
    (Pawn|SetControlRotation (Pawn|GetController) (Math|Conversions|RotationFromXVector (Math|Vector|MakeVector (stale Input|AxisEvents|InputAxisFireRight AxisValue) AxisValue 0.0)))
    (Default|PullTrigger _weapon)
    (else
      (Default|ReleaseTrigger _weapon))))

(event Input|AxisEvents|InputAxisFireRight
  (params (AxisValue :type Float%20%28single-precision%29))
  (bind _weapon (Variables|Default|GetWeapon))
  ;[1 1 1] Rotation
  (if (> (Math|Vector|VectorLength (Math|Vector|MakeVector AxisValue (stale Input|AxisEvents|InputAxisFireUp AxisValue) 0.0)) 0.25)
    (Pawn|SetControlRotation (Pawn|GetController) (Math|Conversions|RotationFromXVector (Math|Vector|MakeVector AxisValue (stale Input|AxisEvents|InputAxisFireUp AxisValue) 0.0)))
    (Default|PullTrigger _weapon)
    (else
      (Default|ReleaseTrigger _weapon))))

(fn ConstructionScript)
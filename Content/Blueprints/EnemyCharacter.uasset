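; Enemy character that deals repeated damage to an overlapping HeroCharacter and shows its own health through body color.
; A construction-script dynamic material drives BodyColor, which AffectHealth lerps by remaining health before destroying the actor on death.
; Overlap start sets a looping DamageTheHero timer at the attack rate, targeting the Hero object although that event lives here.
; Overlap end clears that timer on the enemy itself.
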(event Custom|DamageTheHero
  (Default|AffectHealth (Variables|Default|GetHero) (Variables|Default|GetDamage)))

(event EventBeginPlay
  (Variables|Default|SetEnemyColor "(R=1.000000,G=0.000000,B=0.087898,A=1.000000)"))

(event Collision|EventActorBeginOverlap
  (params (OtherActor :type Actor%20Object%20Reference))
  (bind _ashero_character (Utilities|Casting|CastToHeroCharacter OtherActor))
  (bind _output_get (Variables|Default|SetHero _ashero_character))
  (Utilities|Time|SetTimerbyFunctionName _output_get "DamageTheHero" (/ 1.0 (Variables|Default|GetAttacksPerSecond)) true))

(event Collision|EventActorEndOverlap
  (params (OtherActor :type Actor%20Object%20Reference))
  (if (== OtherActor (Variables|Default|GetHero))
    (Utilities|Time|ClearTimerbyFunctionName 0 "DamageTheHero")))

(event EventTick
  (params (DeltaSeconds :type Float%20%28single-precision%29)))

(event EventAffectHealth
  (params (Delta :type Float%20%28single-precision%29))
  (bind _health (Variables|Default|GetHealth))
  (bind _returnvalue (/ _health 1e+02))
  (bind _returnvalue_2 (Math|Color|Lerp(LinearColor) "(R=0.541667,G=0.000000,B=0.043813,A=1.000000)" "(R=1.000000,G=0.125397,B=0.000000,A=1.000000)" _returnvalue))
  (Class|BaseCharacter|CalculateHealth Delta)
  (Variables|Default|SetEnemyColor _returnvalue_2)
  (Rendering|Material|SetVectorParameterValue (Variables|Default|GetDynamat) "BodyColor" _returnvalue_2 :!class /Script/Engine.MaterialInstanceDynamic)
  (Development|PrintString (Utilities|String|ToString(Float) _returnvalue))
  (if (Variables|Default|GetIsDead)
    (Actor|DestroyActor)))

(fn ConstructionScript
  (bind _returnvalue (Rendering|Material|CreateDynamicMaterialInstance (Variables|Character|GetMesh) 0 0 "None" :!class /Script/Engine.PrimitiveComponent))
  (bind _output_get (Variables|Default|SetDynaMat _returnvalue))
  (Rendering|Material|SetVectorParameterValue _output_get "BodyColor" (Variables|Default|GetEnemyColor) :!class /Script/Engine.MaterialInstanceDynamic))